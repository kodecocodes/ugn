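; BP_Player is the player ship in a shoot 'em up, moved by horizontal and vertical input axes with swept world offsets.
; Holding Shoot spawns BP_Bullet at a spawn point, with a Delay-based cooldown flag limiting fire rate.
; Overlapping a BP_Enemy triggers Explode, which disables input and collision, hides the ship, plays explosion effects and reloads GameMap after a short delay.
; Escape quits the game.
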(event OnComponentBeginOverlap(Hitbox)
  (params (OverlappedComponent :type Primitive%20Component%20Object%20Reference) (OtherActor :type Actor%20Object%20Reference) (OtherComp :type Primitive%20Component%20Object%20Reference) (OtherBodyIndex :type Integer) (bFromSweep :type Boolean) (SweepResult :type Hit%20Result%20Structure%20%28by%20ref%29))
  (Utilities|Casting|CastToBP_Enemy OtherActor)
  (CallFunction|Explode))

(event Custom|Explode
  (Utilities|FlowControl|Sequence
    (:then_0
      (Input|DisableInput (Game|GetPlayerController 0))
      (Collision|SetCollisionEnabled (Variables|Default|GetHitbox) "NoCollision"))
    (:then_1
      (Rendering|SetVisibility (Variables|Default|GetShipMesh) false false)
      (Components|Activation|Deactivate (Variables|Default|GetParticleSystem)))
    (:then_2
      (Effects|SpawnEmitteratLocation "/Game/ShootEmUp/ParticleSystems/PS_Explosion.PS_Explosion" (Transformation|GetActorLocation))
      (Audio|PlaySound2D "/Game/ShootEmUp/Audio/S_Pop.S_Pop" 1.0 1.0 0.0 0 0))
    (:then_3
      (Utilities|FlowControl|Delay 2.0)
      (Game|OpenLevel(byName) "GameMap"))))

(event EventBeginPlay)

(event Collision|EventActorBeginOverlap
  (params (OtherActor :type Actor%20Object%20Reference)))

(event EventTick
  (params (DeltaSeconds :type Float%20%28single-precision%29)))

(event Input|AxisEvents|InputAxisMoveHorizontal
  (params (AxisValue :type Float%20%28single-precision%29))
  (Transformation|AddActorWorldOffset (* "1.000000, 0, 0" (* AxisValue (Variables|Default|GetMoveSpeed) (Utilities|Time|GetWorldDeltaSeconds))) true))

(event Input|AxisEvents|InputAxisMoveVertical
  (params (AxisValue :type Float%20%28single-precision%29))
  (Transformation|AddActorWorldOffset (* "0.000000,-1.000000,0.000000" (* AxisValue (Variables|Default|GetMoveSpeed) (Utilities|Time|GetWorldDeltaSeconds))) true))

(event Input|AxisEvents|InputAxisShoot
  (params (AxisValue :type Float%20%28single-precision%29))
  (if (and (!= AxisValue 0.0) (Variables|Default|GetCanShoot))
    (Game|SpawnActorfromClass "/Game/ShootEmUp/Blueprints/BP_Bullet.BP_Bullet_C" (Math|Transform|MakeTransform (Transformation|GetWorldLocation (Variables|Default|GetBulletSpawnPoint)) "0, 0, 0" "1,1,1") "Undefined" 0 0)
    (Variables|Default|SetCanShoot false)
    (Audio|PlaySound2D "/Game/ShootEmUp/Audio/S_Shoot.S_Shoot" 1.0 1.0 0.0 0 0)
    (Utilities|FlowControl|Delay (Variables|Default|GetShootCooldown))
    (Variables|Default|SetCanShoot true)))

(event Input|KeyboardEvents|Escape
  (params (Key :type Key%20Structure))
  (:Pressed
    (Game|QuitGame 0 "Quit")))

(fn ConstructionScript)