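; BP_Bullet is a projectile actor for a shoot-em-up that destroys enemies it hits.
; Each tick it moves along world X at MoveSpeed with a swept offset, and it removes itself after LiveDuration seconds.
; When its Hitbox overlaps a BP_Enemy, it calls Explode on that enemy and destroys itself, ignoring other actors.
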(event OnComponentBeginOverlap(Hitbox)
  (params (OverlappedComponent :type Primitive%20Component%20Object%20Reference) (OtherActor :type Actor%20Object%20Reference) (OtherComp :type Primitive%20Component%20Object%20Reference) (OtherBodyIndex :type Integer) (bFromSweep :type Boolean) (SweepResult :type Hit%20Result%20Structure%20%28by%20ref%29))
  (bind _asbp_enemy (Utilities|Casting|CastToBP_Enemy OtherActor))
  (Default|Explode _asbp_enemy)
  (Actor|DestroyActor))

(event EventBeginPlay
  (Utilities|FlowControl|Delay (Variables|Default|GetLiveDuration))
  (Actor|DestroyActor))

(event Collision|EventActorBeginOverlap
  (params (OtherActor :type Actor%20Object%20Reference)))

(event EventTick
  (params (DeltaSeconds :type Float%20%28single-precision%29))
  (Transformation|AddActorWorldOffset (* "1.000000, 0, 0" (* DeltaSeconds (Variables|Default|GetMoveSpeed))) true))

(fn ConstructionScript)