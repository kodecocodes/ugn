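; BP_EnemySpawner repeatedly spawns BP_Enemy actors in the shoot 'em up game.
; On Tick, while CanSpawn is true, it spawns an enemy with a fixed rotation at a random point inside the SpawnZone box, centered on the actor's location.
; It then clears CanSpawn and uses a Delay of SpawnCooldown to set it again, pacing the spawns.
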(event EventBeginPlay)

(event Collision|EventActorBeginOverlap
  (params (OtherActor :type Actor%20Object%20Reference)))

(event EventTick
  (params (DeltaSeconds :type Float%20%28single-precision%29))
  (if (Variables|Default|GetCanSpawn)
    (Game|SpawnActorfromClass "/Game/ShootEmUp/Blueprints/BP_Enemy.BP_Enemy_C" (Math|Transform|MakeTransform (Math|Random|RandomPointinBoundingBox (Transformation|GetActorLocation) (Components|Box|GetScaledBoxExtent (Variables|Default|GetSpawnZone))) "0,180.000000, 0" "1,1,1") "Undefined" 0 0)
    (Variables|Default|SetCanSpawn false)
    (Utilities|FlowControl|Delay (Variables|Default|GetSpawnCooldown))
    (Variables|Default|SetCanSpawn true)))

(fn ConstructionScript)