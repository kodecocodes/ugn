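; BP_Enemy is a shoot 'em up enemy ship that flies steadily along negative X at its move speed, using swept movement.
; On begin play it creates a dynamic ship material with a random hue shift, so each ship gets its own color.
; Explode spawns an explosion particle tinted with that same hue, destroys the actor and plays a pop sound.
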(event EventBeginPlay
  (bind _returnvalue (Rendering|Material|CreateDynamicMaterialInstance "/Game/ShootEmUp/Materials/M_BaseShip.M_BaseShip" "None" :!class /Script/Engine.KismetMaterialLibrary))
  (bind _output_get (Variables|Default|SetShipMaterial _returnvalue))
  (Rendering|Material|SetScalarParameterValue _output_get "HueShift" (Math|Random|RandomFloatinRange 0.0 1.0) :!class /Script/Engine.MaterialInstanceDynamic)
  (Rendering|Material|SetMaterial (Variables|Default|GetShipMesh) 0 (Variables|Default|GetShipMaterial)))

(event Collision|EventActorBeginOverlap
  (params (OtherActor :type Actor%20Object%20Reference)))

(event EventTick
  (params (DeltaSeconds :type Float%20%28single-precision%29))
  (Transformation|AddActorWorldOffset (* "-1.000000, 0, 0" (* DeltaSeconds (Variables|Default|GetMoveSpeed))) true))

(fn ConstructionScript)

(fn Explode
  (bind _returnvalue (Effects|SpawnEmitteratLocation "/Game/ShootEmUp/ParticleSystems/PS_Explosion.PS_Explosion" (Transformation|GetActorLocation)))
  (bind _returnvalue_2 (Rendering|Material|GetScalarParameterValue (Variables|Default|GetShipMaterial) "HueShift" :!class /Script/Engine.MaterialInstanceDynamic))
  (Effects|Components|ParticleSystem|SetFloatParameter _returnvalue "HueShift" _returnvalue_2)
  (Actor|DestroyActor)
  (Audio|PlaySound2D "/Game/ShootEmUp/Audio/S_Pop.S_Pop" 1.0 1.0 0.0 0 0))