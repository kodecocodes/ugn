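; Puzzle game manager that runs level selection, loading and completion progress.
; On play it creates a save object, restores the levels array from an existing save slot and shows a level select widget.
; Loading a level hides the menu and streams that level in as an instance by name.
; Completing one flags it done, unloads the instance, refreshes the menu and writes progress back to the slot.
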(event EventBeginPlay
  (Utilities|FlowControl|Sequence
    (:then_0
      (bind _returnvalue (SaveGame|CreateSaveGameObject "/Game/Puzzle/Blueprints/BP_SaveGame.BP_SaveGame_C"))
      (Variables|Default|SetSaveGame _returnvalue))
    (:then_1
      (bind _returnvalue_2 (SaveGame|DoesSaveGameExist (Variables|Default|GetSaveSlotName)))
      (if _returnvalue_2
        (CallFunction|LoadSaveData)))
    (:then_2
      (CallFunction|CreateLevelSelectMenu))))

(fn ConstructionScript)

(fn CreateLevelSelectMenu
  (bind _returnvalue (UserInterface|CreateWidget "/Game/Puzzle/UI/WBP_LevelSelectMenu.WBP_LevelSelectMenu_C" 0 self))
  (bind _output_get (Variables|Default|SetLevelSelectMenu _returnvalue))
  (Default|CreateLevelButtons _output_get)
  (Default|RefreshButtons _output_get)
  (UserInterface|Viewport|AddtoViewport _output_get 0))

(fn LoadSaveData
  (bind _returnvalue (SaveGame|LoadGamefromSlot (Variables|Default|GetSaveSlotName)))
  (bind _asbp_save_game (Utilities|Casting|CastToBP_SaveGame _returnvalue))
  (Variables|Default|SetLevels (Variables|/Game/Puzzle/Blueprints/BP_SaveGame.BP_SaveGame_C|GetLevels _asbp_save_game)))

(fn LoadLevel
  (params (NewLevelIndex :type Integer))
  (Utilities|FlowControl|Sequence
    (:then_0
      (Widget|RemovefromParent (Variables|Default|GetLevelSelectMenu))
      (Variables|Default|SetCurrentLevelIndex NewLevelIndex))
    (:then_1
      (bind _returnvalue (Class|LevelStreamingKismet|LoadLevelInstance (.name (Utilities|Array|Get(acopy) (Variables|Default|GetLevels) (Variables|Default|GetCurrentLevelIndex))) "0, 0, 0" "0, 0, 0"))
      (Variables|Default|SetCurrentLevel _returnvalue))))

(fn CompleteLevel
  (bind _levelselectmenu (Variables|Default|GetLevelSelectMenu))
  (bind _currentlevel (Variables|Default|GetCurrentLevel))
  (Utilities|FlowControl|Sequence
    (:then_0
      (Utilities|Struct|SetmembersinSLevelData (Utilities|Array|Get(acopy) (Variables|Default|GetLevels) (Variables|Default|GetCurrentLevelIndex)) true))
    (:then_1
      (Utilities|IsValid _currentlevel
        (:Is%20Valid
          (Variables|/Script/Engine.LevelStreaming|SetbShouldBeLoaded _currentlevel false))))
    (:then_2
      (UserInterface|Viewport|AddtoViewport _levelselectmenu 0)
      (Default|RefreshButtons _levelselectmenu))
    (:then_3
      (CallFunction|SaveLevelData))))

(fn SaveLevelData
  (bind _savegame (Variables|Default|GetSaveGame))
  (Variables|/Game/Puzzle/Blueprints/BP_SaveGame.BP_SaveGame_C|SetLevels _savegame (Variables|Default|GetLevels))
  (SaveGame|SaveGametoSlot _savegame (Variables|Default|GetSaveSlotName)))