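; BP_CubeObstacle is a puzzle obstacle that moves when its linked switch activates.
; On BeginPlay it binds DeactivateObstacle to the LinkedSwitch's activation event.
; That event stores the Collision's relative location, then plays a timeline that lerps it to TargetLocation without sweeping.
; Its IsDeactivated guard sets the flag to false rather than true, so this graph never blocks repeat triggers.
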(event EventBeginPlay
  (EventDispatchers|BindEventtoActivateSwitch (Variables|Default|GetLinkedSwitch) (delegate EventDeactivateObstacle)))

(event Collision|EventActorBeginOverlap
  (params (OtherActor :type Actor%20Object%20Reference)))

(event EventTick
  (params (DeltaSeconds :type Float%20%28single-precision%29)))

(event EventDeactivateObstacle
  (if (not (Variables|Default|GetIsDeactivated))
    (Utilities|FlowControl|Sequence
      (:then_0
        (Variables|Default|SetIsDeactivated false)
        (Variables|Default|SetStartLocation (Variables|/Script/Engine.SceneComponent|GetRelativeLocation (Variables|Default|GetCollision))))
      (:then_1
        (bind _alpha (Timeline|MoveMeshTimeline Play)
          (:Update
            (Transformation|SetRelativeLocation (Variables|Default|GetCollision) (Math|Vector|Lerp(Vector) (Variables|Default|GetStartLocation) (Variables|Default|GetTargetLocation) _alpha) false false)))))))

(fn ConstructionScript)