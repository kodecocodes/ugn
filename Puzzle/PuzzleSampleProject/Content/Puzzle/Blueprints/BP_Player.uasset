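; BP_Player is the puzzle game's player pawn, which controls a BP_Muffin unit by click-to-move.
; On BeginPlay it possesses itself with the first player controller and stores the first BP_Muffin found as the controlled unit.
; The Move input traces under the cursor and sends that unit to the hit location with AIMoveTo.
; Escape quits the game.
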(event EventBeginPlay
  (Pawn|Possess (Game|GetPlayerController 0) self)
  (bind _outactors (Actor|GetAllActorsOfClass "/Game/Puzzle/Characters/Muffin/Blueprints/BP_Muffin.BP_Muffin_C"))
  (Variables|Default|SetControlledUnit (Utilities|Array|Get(acopy) _outactors)))

(event Input|ActionEvents|InputActionMove
  (params (Key :type Key%20Structure))
  (bind _returnvalue (Game|GetPlayerController 0))
  (bind (_hitresult _returnvalue_2) (Game|Player|GetHitResultUnderCursorbyChannel _returnvalue "TraceTypeQuery3" true))
  (:Pressed
    (if _returnvalue_2
      (AI|AIMoveTo (Variables|Default|GetControlledUnit) (.Location (Collision|BreakHitResult _hitresult)) 0 5.0 false))))

(event Input|KeyboardEvents|Escape
  (params (Key :type Key%20Structure))
  (:Pressed
    (Game|QuitGame 0 "Quit")))

(fn ConstructionScript)