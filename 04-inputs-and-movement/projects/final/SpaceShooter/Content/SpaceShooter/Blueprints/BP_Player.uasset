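; BP_Player is the player Blueprint for the SpaceShooter game and currently handles only movement.
; The MoveUp and MoveRight axis inputs offset the actor in world space along negative Y and positive X, scaled by Speed and world delta seconds.
; Offsets are applied without sweep, so movement ignores collision; BeginPlay, overlap, Tick and the construction script are empty.
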(event EventBeginPlay)

(event Collision|EventActorBeginOverlap
  (params (OtherActor :type Actor%20Object%20Reference)))

(event EventTick
  (params (DeltaSeconds :type Float%20%28single-precision%29)))

(event Input|AxisEvents|InputAxisMoveUp
  (params (AxisValue :type Float%20%28single-precision%29))
  (Transformation|AddActorWorldOffset (* "0,-1.000000, 0" (* AxisValue (Variables|Default|GetSpeed) (Utilities|Time|GetWorldDeltaSeconds)))))

(event Input|AxisEvents|InputAxisMoveRight
  (params (AxisValue :type Float%20%28single-precision%29))
  (Transformation|AddActorWorldOffset (* "1.000000,0.000000, 0" (* AxisValue (Variables|Default|GetSpeed) (Utilities|Time|GetWorldDeltaSeconds)))))

(fn ConstructionScript)